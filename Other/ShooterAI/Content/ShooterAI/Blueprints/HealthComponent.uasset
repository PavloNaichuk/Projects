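; Actor component that gives its owner a health pool and tracks damage and death.
; On BeginPlay it resets Health to StartingHealth and binds to the owner's OnTakeAnyDamage.
; Each hit fires the OnDamageTaken dispatcher before subtracting damage clamped at zero, then fires OnDied whenever IsDead finds health depleted.
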(event `self.ReceiveBeginPlay`
  (set `self.Health` (`self.StartingHealth`))
  (add `Actor.OnTakeAnyDamage` (`self.GetOwner`) (delegate `EventOnDamageTaken`)))

(event `EventOnDamageTaken`
  (params (DamagedActor :type "Actor Object Reference") (Damage :type "Float (double-precision)") (DamageType :type "DamageType Object Reference") (InstigatedBy :type "Controller Object Reference") (DamageCauser :type "Actor Object Reference"))
  (`self.OnDamageTaken`)
  (set `self.Health` (`KismetMathLibrary.FMax` (- (`self.Health`) Damage)))
  (if (`self.IsDead`)
    (`self.OnDied`)))

(fn `IsDead`
  (returns (Dead :type Boolean))
  (return (<= (`self.Health`) 0.0)))