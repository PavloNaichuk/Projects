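; AI controller for guard enemies that turns sight and hearing perception into combat states.
; It runs Guard_BT on Guard_BB, storing the spawn location, and state setters write blackboard keys and notify the pawn.
; Seeing a living player triggers Attacking, while a dead non-player actor triggers Seeking.
; Alert or gunshot sounds trigger Seeking and other noises Investigate, with move targets projected onto the navmesh.
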(event `self.ReceiveBeginPlay`
  (bind _blackboardcomponent (`self.UseBlackboard` "/Game/ShooterAI/Blueprints/AI/Guard_BB.Guard_BB"))
  (set `self.BB` _blackboardcomponent)
  (`self.RunBehaviorTree` "/Game/ShooterAI/Blueprints/AI/Guard_BT.Guard_BT")
  (`BlackboardComponent.SetValueAsVector` (`self.BB`) "SpawnLocation" (`self.K2_GetActorLocation` (`self.K2_GetPawn`))))

(event `self.ReceiveTick`
  (params (DeltaSeconds :type "Float (single-precision)")))

(event `self.AIPerception.OnPerceptionUpdated`
  (params (UpdatedActors :type "Array of Actor Object Reference (by ref)"))
  (for _array_element UpdatedActors
    (bind _info (`AIPerceptionComponent.GetActorsPerception` (`self.AIPerception`) _array_element))
    (bind (_target _lastsensedstimuli) (break `ActorPerceptionBlueprintInfo` _info))
    (set `self.LastSeenActor` _target)
    (for _array_element_2 _lastsensedstimuli
      (bind _output_get (set `self.LastSeenStimuli` _array_element_2))
      (bind _returnvalue (`AIPerceptionSystem.GetSenseClassForStimulus` _output_get))
      (if (== _returnvalue "/Script/AIModule.AISense_Sight")
        (`self.ProcessLastVision`)
        (elif (== _returnvalue "/Script/AIModule.AISense_Hearing")
          (`self.ProcessLastHearing`))))))

(fn `GetAttackRange`
  (returns (Range :type "Float (double-precision)"))
  (return 0.0))

(fn `GetCombatState`
  (returns (NewParam :type "/Game/ShooterAI/Blueprints/AI/ECombatState Enum"))
  (return (cast `/Game/ShooterAI/Blueprints/AI/ECombatState` (`BlackboardComponent.GetValueAsEnum` (`self.BB`) (`self.CombatStateKey`)))))

(fn `GetControlledGuard`
  (returns (Guard :type "/Game/ShooterAI/Blueprints/AI/Guard_Char Object Reference"))
  (bind _asguard_char (cast `/Game/ShooterAI/Blueprints/AI/Guard_Char` (`self.K2_GetPawn`)))
  (return _asguard_char))

(fn `GetHasValidWeapon`
  (returns (HasWeapon :type Boolean) (Weapon :type "/Game/ShooterAI/Blueprints/Weapons/Base/WeaponBase Object Reference"))
  (return false null))

(fn `GetIsDead`
  (returns (IsDead :type Boolean))
  (return false))

(fn `GetPatrolRoute`
  (returns (Route :type "/Game/ShooterAI/Blueprints/AI/PatrolRouteBase Object Reference"))
  (return null))

(fn `GetTeamID`
  (returns (TeamID :type Integer))
  (return 0))

(fn `ProcessLastHearing`
  (bind (_lastseenstimuli_age _lastseenstimuli_expirationage _lastseenstimuli_strength _lastseenstimuli_stimuluslocation _lastseenstimuli_receiverlocation _lastseenstimuli_tag _lastseenstimuli_bsuccessfullysensed) (break `AIStimulus` (`self.LastSeenStimuli`)))
  (bind _projectedlocation (`NavigationSystemV1.K2_ProjectPointToNavigation` _lastseenstimuli_stimuluslocation null null (50.0 50.0 200.0)))
  (if _lastseenstimuli_bsuccessfullysensed
    (if (or (== _lastseenstimuli_tag "Alert") (== _lastseenstimuli_tag "Gunshot"))
      (`self.SetCombatStateSeeking` _projectedlocation)
      (else
        (`self.SetCombatStateInvestigate` _lastseenstimuli_stimuluslocation _projectedlocation)))))

(fn `ProcessLastVision`
  (bind (_lastseenstimuli_age _lastseenstimuli_expirationage _lastseenstimuli_strength _lastseenstimuli_stimuluslocation) (break `AIStimulus` (`self.LastSeenStimuli`)))
  (bind _lastseenactor (`self.LastSeenActor`))
  (if (`KismetSystemLibrary.DoesImplementInterface` _lastseenactor "/Game/ShooterAI/Blueprints/AI/AIHelper_BPI.AIHelper_BPI_C")
    (bind _teamid (message `/Game/ShooterAI/Blueprints/AI/AIHelper_BPI.GetTeamID` _lastseenactor))
    (if (== _teamid 0)
      (bind _isdead (message `/Game/ShooterAI/Blueprints/AI/AIHelper_BPI.GetIsDead` (`self.LastSeenActor`)))
      (if (not _isdead)
        (`self.SetCombatStateAttacking` (`self.LastSeenActor`)))
      (else
        (bind _isdead_2 (message `/Game/ShooterAI/Blueprints/AI/AIHelper_BPI.GetIsDead` (`self.LastSeenActor`)))
        (if _isdead_2
          (`self.SetCombatStateSeeking` _lastseenstimuli_stimuluslocation))))))

(fn `SetCombatStateAttacking`
  (params (Enemy :type "Actor Object Reference"))
  (bind _returnvalue (enumliteral `/Game/ShooterAI/Blueprints/AI/ECombatState` "NewEnumerator3"))
  (`BlackboardComponent.SetValueAsEnum` (`self.BB`) (`self.CombatStateKey`) _returnvalue)
  (`BlackboardComponent.SetValueAsObject` (`self.BB`) "EnemyTarget" Enemy)
  (message `/Game/ShooterAI/Blueprints/AI/AIHelper_BPI.NotifyStateChanged` (`self.K2_GetPawn`) _returnvalue))

(fn `SetCombatStateInvestigate`
  (params (POI :type "Vector Structure") (MoveTo :type "Vector Structure"))
  (bind _returnvalue (enumliteral `/Game/ShooterAI/Blueprints/AI/ECombatState` "NewEnumerator1"))
  (`BlackboardComponent.SetValueAsEnum` (`self.BB`) (`self.CombatStateKey`) _returnvalue)
  (`BlackboardComponent.SetValueAsVector` (`self.BB`) (`self.MoveToKey`) MoveTo)
  (`BlackboardComponent.SetValueAsVector` (`self.BB`) (`self.POI_Key`) POI)
  (message `/Game/ShooterAI/Blueprints/AI/AIHelper_BPI.NotifyStateChanged` (`self.K2_GetPawn`) _returnvalue))

(fn `SetCombatStatePassive`
  (bind _returnvalue (enumliteral `/Game/ShooterAI/Blueprints/AI/ECombatState` "NewEnumerator0"))
  (`BlackboardComponent.SetValueAsEnum` (`self.BB`) (`self.CombatStateKey`) _returnvalue)
  (message `/Game/ShooterAI/Blueprints/AI/AIHelper_BPI.NotifyStateChanged` (`self.K2_GetPawn`) _returnvalue))

(fn `SetCombatStateSeeking`
  (params (Search :type "Vector Structure"))
  (bind _returnvalue (enumliteral `/Game/ShooterAI/Blueprints/AI/ECombatState` "NewEnumerator2"))
  (`BlackboardComponent.SetValueAsEnum` (`self.BB`) (`self.CombatStateKey`) _returnvalue)
  (`BlackboardComponent.SetValueAsVector` (`self.BB`) (`self.MoveToKey`) Search)
  (message `/Game/ShooterAI/Blueprints/AI/AIHelper_BPI.NotifyStateChanged` (`self.K2_GetPawn`) _returnvalue))

(fn `UserConstructionScript`)