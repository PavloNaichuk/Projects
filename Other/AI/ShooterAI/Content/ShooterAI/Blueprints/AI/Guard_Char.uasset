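; Guard AI character that carries a weapon, follows an assigned patrol route and belongs to a fixed team.
; On BeginPlay it spawns its controller and attaches a spawned weapon to the hand grip socket.
; It forwards aiming and state changes to its anim Blueprint, tunes movement by AI state and exposes combat queries.
; When its health component reports death, the mesh ragdolls and capsule collision is disabled.
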(event `self.ReceiveBeginPlay`
  (`self.SpawnDefaultController`)
  (bind _returnvalue (`|SpawnActorFromClass` (`self.WeaponClass`) (`KismetMathLibrary.MakeTransform` (0.0 0.0 0.0)) "AlwaysSpawn" "OverrideRootScale" self self))
  (set `self.MyWeapon` _returnvalue)
  (`self.K2_AttachToComponent` _returnvalue (`self.Mesh`) "GripPoint" "SnapToTarget" "SnapToTarget" "KeepWorld" true))

(event `/Game/ShooterAI/Blueprints/AI/AIHelper_BPI.ChangeAimingMode`
  (params (Aiming :type Boolean))
  (message `/Game/ShooterAI/Blueprints/AI/AIHelper_BPI.ChangeAimingMode` (`self.GetAnimBlueprint`) Aiming))

(event `/Game/ShooterAI/Blueprints/AI/AIHelper_BPI.NotifyStateChanged`
  (params (NewState :type "/Game/ShooterAI/Blueprints/AI/ECombatState Enum" :default "NewEnumerator0"))
  (message `/Game/ShooterAI/Blueprints/AI/AIHelper_BPI.NotifyStateChanged` (`self.GetAnimBlueprint`) NewState))

(event `self.HealthComponent.OnDied`
  (bind _mesh (`self.Mesh`))
  (`PrimitiveComponent.SetCollisionProfileName` _mesh "Ragdoll" true)
  (`SkeletalMeshComponent.SetAllBodiesSimulatePhysics` _mesh true)
  (`PrimitiveComponent.WakeAllRigidBodies` _mesh)
  (`PrimitiveComponent.SetCollisionEnabled` (`self.CapsuleComponent`) "NoCollision"))

(event `TryStartShooting`
  (bind _myweapon (`self.MyWeapon`)
    (:`then`
      (`/Game/ShooterAI/Blueprints/Weapons/Base/WeaponBase.OnFireBegin` _myweapon))
    (:`else`)))

(fn `GetAnimBlueprint`
  (returns (AnimBP :type "/Game/ShooterAI/Characters/Mannequin/Animations/ThirdPerson_AnimBP Object Reference"))
  (bind _asthird_person_anim_bp (cast `/Game/ShooterAI/Characters/Mannequin/Animations/ThirdPerson_AnimBP` (`SkeletalMeshComponent.GetAnimInstance` (`self.Mesh`))))
  (return _asthird_person_anim_bp))

(fn `GetAttackRange`
  (returns (Range :type "Float (double-precision)"))
  (return (`self.Range`)))

(fn `GetHasValidWeapon`
  (returns (HasWeapon :type Boolean) (Weapon :type "/Game/ShooterAI/Blueprints/Weapons/Base/WeaponBase Object Reference"))
  (bind _myweapon (`self.MyWeapon`))
  (return (`KismetSystemLibrary.IsValid` _myweapon) _myweapon))

(fn `GetIsDead`
  (returns (IsDead :type Boolean))
  (return (`/Game/ShooterAI/Blueprints/HealthComponent.IsDead` (`self.HealthComponent`))))

(fn `GetPatrolRoute`
  (returns (Route :type "/Game/ShooterAI/Blueprints/AI/PatrolRouteBase Object Reference"))
  (return (`self.MyPatrol`)))

(fn `GetTeamID`
  (returns (TeamID :type Integer))
  (return 1))

(fn `ModifyMovementSpeed`
  (params (Index :type "/Game/ShooterAI/Blueprints/AI/ECombatState Enum" :default "NewEnumerator0"))
  (`|ExecutionSequence`
    (:`then_0`
      (set `CharacterMovementComponent.MaxWalkSpeed` (select `/Game/ShooterAI/Blueprints/AI/ECombatState` Index :`NewEnumerator0` 165.0 :`NewEnumerator1` 165.0 :`NewEnumerator2` 400.0 :`NewEnumerator3` 400.0 :!type "Float (single-precision)") (`self.CharacterMovement`)))
    (:`then_1`
      (set `CharacterMovementComponent.MaxAcceleration` (select `/Game/ShooterAI/Blueprints/AI/ECombatState` Index :`NewEnumerator0` 800.0 :`NewEnumerator1` 800.0 :`NewEnumerator2` 1000.0 :`NewEnumerator3` 1000.0 :!type "Float (single-precision)") (`self.CharacterMovement`)))
    (:`then_2`
      (set `CharacterMovementComponent.BrakingDecelerationWalking` (select `/Game/ShooterAI/Blueprints/AI/ECombatState` Index :`NewEnumerator0` 700.0 :`NewEnumerator1` 700.0 :`NewEnumerator2` 800.0 :`NewEnumerator3` 800.0 :!type "Float (single-precision)") (`self.CharacterMovement`)))))

(fn `UserConstructionScript`)