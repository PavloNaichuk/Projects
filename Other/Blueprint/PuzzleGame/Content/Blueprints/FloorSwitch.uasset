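; Floor switch that activates its AffectedActors while a PuzzleCharacter stands in its box trigger.
; Overlap begin and end send ActivateMessage and DeactivateMessage through SwitchInterface to each listed actor implementing it.
; A timeline offsets the switch mesh's height from its starting position, playing on entry.
; The timeline reverses inside the exit loop, so the mesh returns only when an affected actor implements the interface.
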(event `self.ReceiveBeginPlay`
  (set `self.InitialSwitchLocation` (`SceneComponent.K2_GetComponentLocation` (`self.SwitchMesh`))))

(event `self.Box.OnComponentBeginOverlap`
  (params (OverlappedComponent :type "PrimitiveComponent Object Reference") (OtherActor :type "Actor Object Reference") (OtherComp :type "PrimitiveComponent Object Reference") (OtherBodyIndex :type Integer) (bFromSweep :type Boolean) (SweepResult :type "HitResult Structure (by ref)"))
  (cast `/Game/Blueprints/Character/PuzzleCharacter` OtherActor)
  (for _array_element (`self.AffectedActors`)
    (if (`KismetSystemLibrary.DoesImplementInterface` _array_element "/Game/Blueprints/SwitchInterface.SwitchInterface_C")
      (message `/Game/Blueprints/SwitchInterface.Activate` _array_element)))
  (bind (_direction _switchelevation) (`Timeline|SwitchTimeline` :!label _label)
    (:`Update`
      (`SceneComponent.K2_SetWorldLocation` (`self.SwitchMesh`) (`KismetMathLibrary.MakeVector` (.x (`self.InitialSwitchLocation`)) (.y (`self.InitialSwitchLocation`)) (+ _switchelevation (.z (`self.InitialSwitchLocation`)))) false false))))

(event `self.Box.OnComponentEndOverlap`
  (params (OverlappedComponent :type "PrimitiveComponent Object Reference") (OtherActor :type "Actor Object Reference") (OtherComp :type "PrimitiveComponent Object Reference") (OtherBodyIndex :type Integer))
  (cast `/Game/Blueprints/Character/PuzzleCharacter` OtherActor)
  (for _array_element (`self.AffectedActors`)
    (if (`KismetSystemLibrary.DoesImplementInterface` _array_element "/Game/Blueprints/SwitchInterface.SwitchInterface_C")
      (message `/Game/Blueprints/SwitchInterface.Deactivate` _array_element)
      (goto _label :!via `Reverse`))))

(fn `UserConstructionScript`)