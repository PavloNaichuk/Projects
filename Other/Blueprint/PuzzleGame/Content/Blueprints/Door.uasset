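; Door actor whose mesh slides vertically when its Activate event fires.
; BeginPlay caches the mesh's starting world location.
; Activate plays a timeline whose DoorElevation track is added to that starting Z on each update, moving the mesh without sweep while X and Y stay fixed.
; The graph contains no reverse or closing logic.
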(event `self.ReceiveBeginPlay`
  (set `self.InitialDoorLocation` (`SceneComponent.K2_GetComponentLocation` (`self.DoorMesh`))))

(event `/Game/Blueprints/SwitchInterface.Activate`
  (bind (_direction _doorelevation) (`Timeline|DoorTimeline`)
    (:`Update`
      (`SceneComponent.K2_SetWorldLocation` (`self.DoorMesh`) (`KismetMathLibrary.MakeVector` (.x (`self.InitialDoorLocation`)) (.y (`self.InitialDoorLocation`)) (+ _doorelevation (.z (`self.InitialDoorLocation`)))) false false))))

(fn `UserConstructionScript`)