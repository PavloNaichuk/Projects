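; Booster is a launch pad that flings a BallPawn upward when it hits the Button component.
; The hit applies a fixed vertical velocity-change impulse to the ball mesh, plays a 2D sound and starts BoosterTimeline.
; The timeline offsets the button's height from the location cached at BeginPlay, with a half-second Delay on its Update output that then reverses it.
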(event `self.ReceiveBeginPlay`
  (set `self.InitialButtonLocation` (`SceneComponent.K2_GetComponentLocation` (`self.Button`))))

(event `self.Button.OnComponentHit`
  (params (HitComponent :type "PrimitiveComponent Object Reference") (OtherActor :type "Actor Object Reference") (OtherComp :type "PrimitiveComponent Object Reference") (NormalImpulse :type "Vector Structure") (Hit :type "HitResult Structure (by ref)"))
  (bind _asball_pawn (cast `/Game/Blueprints/BallPawn` OtherActor))
  (`PrimitiveComponent.AddImpulse` (`/Game/Blueprints/BallPawn.BallMesh` _asball_pawn) (0.0 0.0 800.0) "None" true)
  (`GameplayStatics.PlaySound2D` "/Game/Sounds/GrassHit.GrassHit" 1.0 1.0 0.0 null null)
  (bind (_direction _boosterlaunchelevation) (`Timeline|BoosterTimeline` :!label _label)
    (:`Update`
      (`SceneComponent.K2_SetWorldLocation` (`self.Button`) (`KismetMathLibrary.MakeVector` (.x (`self.InitialButtonLocation`)) (.y (`self.InitialButtonLocation`)) (+ (.z (`self.InitialButtonLocation`)) _boosterlaunchelevation)) false false)
      (`KismetSystemLibrary.Delay` 0.5)
      (goto _label :!via `Reverse`))))

(fn `UserConstructionScript`)