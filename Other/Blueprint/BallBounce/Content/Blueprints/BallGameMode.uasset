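; BallGameMode is a game mode that runs the match state machine for a ball game, starting in Ready.
; SetGameState handles each transition: Countdown resets the timer, Playing fires StartPlaying, and Ooops returns to Ready after a short delay.
; Tick drives the countdown, converting remaining time into a whole-number Count and switching to Playing when it runs out.
; Game Over and Level Completed only store the new state.
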(event `self.ReceiveBeginPlay`
  (set `self.StateOfThegame` "NewEnumerator0"))

(event `self.ReceiveTick`
  (params (DeltaSeconds :type "Float (single-precision)"))
  (if (`|EnumEquality` (`self.StateOfThegame`) "NewEnumerator1")
    (bind _output_get (set `self.Countdown` (- (`self.Countdown`) DeltaSeconds)))
    (if (>= _output_get 2.0)
      (set `self.Count` 3)
      (elif (>= _output_get 1.0)
        (set `self.Count` 2)
        (elif (>= _output_get 0.0)
          (set `self.Count` 1)
          (else
            (`self.SetGameState` "NewEnumerator5")))))))

(event `SetGameState`
  (params (NewParam :type "/Game/Blueprints/StateOfGame Enum" :default "NewEnumerator0"))
  (switch `/Game/Blueprints/StateOfGame` NewParam
    (:`NewEnumerator0`
      (set `self.StateOfThegame` NewParam :!label _label))
    (:`NewEnumerator1`
      (set `self.Countdown` 3.0)
      (set `self.StateOfThegame` "NewEnumerator1"))
    (:`NewEnumerator2`
      (set `self.StateOfThegame` "NewEnumerator2")
      (`KismetSystemLibrary.Delay` 1.5)
      (`self.SetGameState` "NewEnumerator0"))
    (:`NewEnumerator3`
      (goto _label))
    (:`NewEnumerator4`
      (goto _label))
    (:`NewEnumerator5`
      (`self.StartPlaying`)
      (set `self.StateOfThegame` "NewEnumerator5"))))

(fn `UserConstructionScript`)